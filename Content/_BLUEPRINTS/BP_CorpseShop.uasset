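; BP_CorpseShop is a corpse shop trigger, voiced by gravedigger sound cues.
; Entering its box creates the WB_CorpseShop widget for the first player controller and plays a greeting.
; Leaving removes the widget, plays a purchase or disappointment cue based on the BoughtCorpse flag, then clears that flag.
; The overlaps do not filter which actor enters, and sounds play at the world origin.
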(event `self.Box.OnComponentBeginOverlap`
  (params (OverlappedComponent :type "PrimitiveComponent Object Reference") (OtherActor :type "Actor Object Reference") (OtherComp :type "PrimitiveComponent Object Reference") (OtherBodyIndex :type Integer) (bFromSweep :type Boolean) (SweepResult :type "HitResult Structure (by ref)"))
  (bind _returnvalue (`|CreateWidget` "/Game/_WIDGETS/WB_CorpseShop.WB_CorpseShop_C" (`GameplayStatics.GetPlayerController` 0)))
  (`UserWidget.AddToViewport` _returnvalue 0)
  (`GameplayStatics.PlaySoundAtLocation` "/Game/_AUDIO/VoiceLines/SC_GravediggerGreet_Cue.SC_GravediggerGreet_Cue" (0.0 0.0 0.0) (struct) 1.0 1.0 0.0 null null null null))

(event `self.Box.OnComponentEndOverlap`
  (params (OverlappedComponent :type "PrimitiveComponent Object Reference") (OtherActor :type "Actor Object Reference") (OtherComp :type "PrimitiveComponent Object Reference") (OtherBodyIndex :type Integer))
  (`Widget.RemoveFromParent` (stale `self.Box.OnComponentBeginOverlap` _returnvalue))
  (if (`self.boughtCorpse`)
    (`GameplayStatics.PlaySoundAtLocation` "/Game/_AUDIO/VoiceLines/SC_GravediggerPurchase_Cue.SC_GravediggerPurchase_Cue" (0.0 0.0 0.0) (struct) 1.0 1.0 0.0 null null null null)
    (else
      (`GameplayStatics.PlaySoundAtLocation` "/Game/_AUDIO/VoiceLines/SC_GravediggerDisappoint_Cue.SC_GravediggerDisappoint_Cue" (0.0 0.0 0.0) (struct) 1.0 1.0 0.0 null null null null)))
  (set `self.boughtCorpse` false))

(fn `UserConstructionScript`)