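; Skeleton minion character that musters, roams and raids, adding its MinionValue to the resource manager's coins when destroyed.
; Muster issues a move to BP_MusterPoint and immediately starts Roam, which repeats random reachable moves around that point on each success.
; Raid stops roaming, issues a move to BP_RaidPoint and destroys the actor from the immediate exec pin, without waiting for arrival.
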(event `self.ReceiveBeginPlay`
  ;[0.1451 0 0.2431] References
  ;;[0.6 0 1] Get Reference to Resource Manager
  (bind _returnvalue (`GameplayStatics.GetActorOfClass` "/Game/_BLUEPRINTS/BP_ResourceManager.BP_ResourceManager_C"))
  (set `self.ResourceManagerRef` _returnvalue))

(event `Muster`
  ;[0.1451 0 0.2431] Mustering
  ;;[0.6 0 1] Move To Muster Point
  (bind _returnvalue (`GameplayStatics.GetActorOfClass` "/Game/_BLUEPRINTS/BP_MusterPoint.BP_MusterPoint_C"))
  (`|AIMoveTo` self (0.0 0.0 0.0) _returnvalue 0.0
    (:`then`
      ;;[0.6 0 1] Begin Roaming
      (set `self.isRoaming` true)
      (`self.Roam`))))

(event `Roam`
  ;[0.1451 0 0.2431] Roaming
  ;;[0.6 0 1] Check If Roaming
  (if (`self.isRoaming`)
    ;;[0.6 0 1] Roam Randomly In Range
    (bind _returnvalue (`GameplayStatics.GetActorOfClass` "/Game/_BLUEPRINTS/BP_MusterPoint.BP_MusterPoint_C"))
    (`|AIMoveTo` self (`NavigationSystemV1.K2_GetRandomReachablePointInRadius` (`self.K2_GetActorLocation` _returnvalue) 300.0 null null) null
      (:`OnSuccess`
        ;;[0.6 0 1] Repeat
        (`self.Roam`)))))

(event `Raid`
  ;[0.1451 0 0.2431] Raiding
  ;;[0.6 0 1] Turn Off Roaming
  (set `self.isRoaming` false)
  ;;[0.6 0 1] Move To Raid Point
  (bind _returnvalue (`GameplayStatics.GetActorOfClass` "/Game/_BLUEPRINTS/BP_RaidPoint.BP_RaidPoint_C"))
  (`|AIMoveTo` self (0.0 0.0 0.0) _returnvalue 0.0
    (:`then`
      ;;[0.6 0 1] Destroy
      (`self.K2_DestroyActor`))))

(event `self.ReceiveDestroyed`
  (bind _resourcemanagerref (`self.ResourceManagerRef`))
  ;[0.1451 0 0.2431] Reward
  ;;[0.6 0 1] Increase Coin Stockpile Based On Value
  (set `/Game/_BLUEPRINTS/BP_ResourceManager.CurrentCoins` (+ (`/Game/_BLUEPRINTS/BP_ResourceManager.CurrentCoins` _resourcemanagerref) (`self.MinionValue`)) _resourcemanagerref))

(fn `UserConstructionScript`)